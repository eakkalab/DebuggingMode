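; BP_Lever is an interactible lever that the player flips between two positions by dragging while grabbing it.
; Its trigger box toggles visibility of the normal mesh, highlighted mesh and text on overlap begin and end.
; GrabInteract checks vertical aim movement against the current position, calls FlipLever and returns the FocusTarget socket location.
; FlipLever plays or reverses a timeline that rolls the lever, then stores and prints the new state.
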(event `self.BoxTrigger.OnComponentBeginOverlap`
  (params (OverlappedComponent :type "PrimitiveComponent Object Reference") (OtherActor :type "Actor Object Reference") (OtherComp :type "PrimitiveComponent Object Reference") (OtherBodyIndex :type Integer) (bFromSweep :type Boolean) (SweepResult :type "HitResult Structure (by ref)"))
  ;[1 1 1] Set Visibility when a pawn thouches the trigger box
  (`SceneComponent.ToggleVisibility` (`self.Lever`) false :!label _label)
  (`SceneComponent.ToggleVisibility` (`self.LeverHighlighted`) false)
  (`SceneComponent.ToggleVisibility` (`self.TextRender`) false))

(event `self.BoxTrigger.OnComponentEndOverlap`
  (params (OverlappedComponent :type "PrimitiveComponent Object Reference") (OtherActor :type "Actor Object Reference") (OtherComp :type "PrimitiveComponent Object Reference") (OtherBodyIndex :type Integer))
  ;[1 1 1] Set Visibility when a pawn thouches the trigger box
  (goto _label))

(event `FlipLever`
  ;[1 1 1] Animate the lever
  (if (`self.bLeverPosition`)
    (bind (_direction _rollvalue) (`Timeline|RotateLever` :!via `Reverse` :!label _label_2)
      (:`Update`
        (`SceneComponent.K2_SetRelativeRotation` (`self.Lever`) (`KismetMathLibrary.MakeRotator` _rollvalue) false false))
      (:`Finished`
        (bind _output_get (set `self.bLeverPosition` (`|EnumEquality` _direction "Forward")))
        (`KismetSystemLibrary.PrintString` (`KismetStringLibrary.Conv_BoolToString` _output_get))))
    (else
      (goto _label_2))))

(fn `GrabInteract`
  (params (PlayerAimMovement :type "Vector2D Structure") (Interacting :type Boolean))
  (returns (PlayerFocusTarget :type "Vector Structure"))
  (bind (_x _y) (`KismetMathLibrary.BreakVector2D` PlayerAimMovement))
  ;[1 1 1] Drag direction determined by the movement of lever
  (if (or (and (not (`self.bLeverPosition`)) (>= _y 0.5)) (and (<= _y -0.5) (`self.bLeverPosition`)))
    (`self.FlipLever`))
  (return (`SceneComponent.GetSocketLocation` (`self.Lever`) "FocusTarget")))

(fn `UserConstructionScript`)